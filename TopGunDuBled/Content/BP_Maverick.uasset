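; BP_Maverick is a player-controlled actor that fires a hitscan weapon and loses the game on taking any damage.
; While shoot is held, Tick traces forward from the actor on Visibility, with debug drawing, and damages the hit actor every frame.
; A Delay after the damage throttles only the firing sound.
; Any damage received plays an explosion sound, opens LoseMenu, pauses the game and shows the cursor.
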(event `InputAction|shoot`
  (params (Key :type "Key Structure"))
  (:`Pressed`
    (set `self.isShooting?` true))
  (:`Released`
    (set `self.isShooting?` false)))

(event `self.ReceiveTick`
  (params (DeltaSeconds :type "Float (single-precision)"))
  (if (`self.isShooting?`)
    (bind _outhit (`KismetSystemLibrary.LineTraceSingle` :`Start` (`self.K2_GetActorLocation`) :`End` (+ (* (`self.GetActorForwardVector`) 20000.0) (`self.K2_GetActorLocation`)) :`TraceChannel` "TraceTypeQuery1" :`DrawDebugType` "ForDuration"))
    (`GameplayStatics.ApplyDamage` (`.HitActor` (`GameplayStatics.BreakHitResult` _outhit)) 1.0 null null "/Script/Engine.DamageType")
    (`KismetSystemLibrary.Delay` 0.15)
    (`GameplayStatics.PlaySound2D` "/Game/Map/Rifle/Wavs/RifleA_Fire01.RifleA_Fire01" 1.0 1.0 0.0 null null)))

(event `self.ReceiveAnyDamage`
  (params (Damage :type "Float (single-precision)") (DamageType :type "DamageType Object Reference") (InstigatedBy :type "Controller Object Reference") (DamageCauser :type "Actor Object Reference"))
  (`GameplayStatics.PlaySoundAtLocation` "/Game/StarterContent/Audio/Explosion01.Explosion01" (`SceneComponent.RelativeLocation` (`self.Mesh`)) (struct) 1.0 1.0 0.0 null null null)
  (bind _returnvalue (`|CreateWidget` "/Game/HUD/LoseMenu.LoseMenu_C"))
  (`UserWidget.AddToViewport` _returnvalue 0)
  (`GameplayStatics.SetGamePaused` true)
  (set `PlayerController.bShowMouseCursor` true (`GameplayStatics.GetPlayerController` 0)))

(fn `UserConstructionScript`)